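; BP_MiniMapManager creates the mobile minimap widget on BeginPlay, shows the mouse cursor and manages the elements displayed on the map.
; Add and remove events take minimap components, spawn each one's chosen widget class centered in the map overlay, and track the pairs in a map.
; ConvertWorldPosToMapPos scales world positions by the scene capture's ortho width and minimap size, swapping axes and flipping vertical.
; Leftover test-button and error-logging nodes never run.
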(event Custom|DeleteActor
  (Actor|DestroyActor (Variables|Default|GetdebugCube)))

(event Custom|AddMiniMapComponent
  (params (minimapComponent :type AC%20Mini%20Map%20Base%20Element%20Object%20Reference))
  (CallFunction|AddMiniMapElement minimapComponent))

(event Custom|RemoveMiniMapComponent
  (params (minimapComponent :type AC%20Mini%20Map%20Base%20Element%20Object%20Reference))
  (if (.ReturnValue (Utilities|Map|Find (Variables|Default|GetminimapComponents) minimapComponent))
    (Class|PanelWidget|RemoveChild (Variables|/Game/ProjetFilRouge/Core/Mobile/MiniMap/WidgetsBlueprints/WBP_MiniMap.WBP_MiniMap_C|GetMapOverlay (Variables|Default|Getminimap)) (.Value (Utilities|Map|Find (Variables|Default|GetminimapComponents) minimapComponent)))
    (Utilities|Map|Remove (Variables|Default|GetminimapComponents) minimapComponent)))

(event EventBeginPlay
  (Variables|/Script/Engine.PlayerController|SetbShowMouseCursor (Game|GetPlayerController 0) true)
  (bind _returnvalue (UserInterface|CreateWidget "/Game/ProjetFilRouge/Core/Mobile/MiniMap/WidgetsBlueprints/WBP_MiniMap.WBP_MiniMap_C" (Game|GetPlayerController 0)))
  (bind _output_get (Variables|Default|Setminimap _returnvalue))
  (UserInterface|Viewport|AddtoPlayerScreen _output_get))

(fn ConstructionScript)

(fn ConvertWorldPostoMapPos
  (params (worldPos :type Vector%202D%20Structure))
  (bind (_x _y) (Math|Vector2D|BreakVector2D worldPos))
  (bind _minimap (Variables|Default|Getminimap))
  (bind _scenecapturecomponent2d (Variables|Default|GetSceneCaptureComponent2D))
  (bind _minimap_2 (Variables|/Game/ProjetFilRouge/Core/Mobile/MiniMap/WidgetsBlueprints/WBP_MiniMap.WBP_MiniMap_C|GetMiniMap _minimap))
  (bind _orthowidth (Variables|/Script/Engine.SceneCaptureComponent2D|GetOrthoWidth _scenecapturecomponent2d))
  (bind _returnvalue (Class|WidgetLayoutLibrary|SlotasCanvasSlot _minimap_2))
  (bind _returnvalue_2 (/ _orthowidth 2.0))
  (bind _returnvalue_3 (Class|CanvasPanelSlot|GetSize _returnvalue))
  (bind _x_2 (Math|Vector2D|BreakVector2D _returnvalue_3))
  (bind _returnvalue_4 (/ _x_2 2.0))
  (return (Math|Vector2D|MakeVector2D (* (/ _y _returnvalue_2) _returnvalue_4) (* (* (/ _x _returnvalue_2) _returnvalue_4) -1.0))))

(fn AddMiniMapElement
  (params (minimapElement :type AC%20Mini%20Map%20Base%20Element%20Object%20Reference))
  (bind _returnvalue (UserInterface|CreateWidget (Variables|/Game/ProjetFilRouge/Core/Mobile/MiniMap/ActorsComponents/AC_MiniMap_BaseElement.AC_MiniMap_BaseElement_C|GetWBP_Element minimapElement) 0 self minimapElement))
  (Utilities|Map|Add (Variables|Default|GetminimapComponents) minimapElement _returnvalue)
  (bind _returnvalue_2 (Class|Overlay|AddChildtoOverlay (Variables|/Game/ProjetFilRouge/Core/Mobile/MiniMap/WidgetsBlueprints/WBP_MiniMap.WBP_MiniMap_C|GetMapOverlay (Variables|Default|Getminimap)) _returnvalue))
  (Layout|GridSlot|SetHorizontalAlignment _returnvalue_2 "HAlign_Center")
  (Layout|GridSlot|SetVerticalAlignment _returnvalue_2 "VAlign_Center"))