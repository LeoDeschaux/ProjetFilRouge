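; Actor component that registers its owner as an element on the mobile minimap.
; On BeginPlay it waits briefly, then finds BP_Mobile_GameManager and adds itself to that manager's MinimapManager.
; It binds to the owner's destruction to remove itself from the MinimapManager, and exposes the same removal as its own event.
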(event Custom|HanddleOnParentDestroy
  (params (DestroyedActor :type Actor%20Object%20Reference))
  (CallFunction|RemovefromMiniMap))

(event Custom|RemoveFromMiniMap
  (bind _returnvalue (Actor|GetActorOfClass "/Game/ProjetFilRouge/Core/Mobile/BP_Mobile_GameManager.BP_Mobile_GameManager_C"))
  (Default|RemoveMiniMapComponent (Variables|/Game/ProjetFilRouge/Core/Mobile/BP_Mobile_GameManager.BP_Mobile_GameManager_C|GetminimapManager _returnvalue) self))

(event EventBeginPlay
  (Game|BindEventtoOnDestroyed (Components|GetOwner) (delegate Custom|HanddleOnParentDestroy))
  (Utilities|FlowControl|Delay 0.2)
  (bind _returnvalue (Actor|GetActorOfClass "/Game/ProjetFilRouge/Core/Mobile/BP_Mobile_GameManager.BP_Mobile_GameManager_C"))
  (Default|AddMiniMapComponent (Variables|/Game/ProjetFilRouge/Core/Mobile/BP_Mobile_GameManager.BP_Mobile_GameManager_C|GetminimapManager _returnvalue) self))