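; AC_MiniMap_Cursor is an actor component that registers itself as an element of the mobile game's minimap.
; On BeginPlay it runs the parent logic, waits briefly, then finds BP_Mobile_GameManager and adds itself to that manager's MinimapManager.
; A RemoveElement event looks up the same manager and unregisters the component from the minimap.
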(event Custom|RemoveElement
  (bind _returnvalue (Actor|GetActorOfClass "/Game/ProjetFilRouge/Core/Mobile/BP_Mobile_GameManager.BP_Mobile_GameManager_C"))
  (Default|RemoveMiniMapComponent (Variables|/Game/ProjetFilRouge/Core/Mobile/BP_Mobile_GameManager.BP_Mobile_GameManager_C|GetminimapManager _returnvalue) self))

(event EventBeginPlay
  (|CallParentFunction)
  (Utilities|FlowControl|Delay 0.2)
  (bind _returnvalue (Actor|GetActorOfClass "/Game/ProjetFilRouge/Core/Mobile/BP_Mobile_GameManager.BP_Mobile_GameManager_C"))
  (Default|AddMiniMapComponent (Variables|/Game/ProjetFilRouge/Core/Mobile/BP_Mobile_GameManager.BP_Mobile_GameManager_C|GetminimapManager _returnvalue) self))