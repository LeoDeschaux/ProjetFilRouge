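; Minimap capture actor for the mobile side of the game, apparently a test of clickable map markers tied to world actors.
; On BeginPlay it shows the cursor, creates the minimap widget and adds a map button to its overlay.
; The button is placed by scaling DebugCube's world position from the scene capture's ortho width to widget size, swapping axes and assuming a world-origin center.
; Clicking the button destroys DebugCube.
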(event Custom|DeleteActor
  (Actor|DestroyActor (Variables|Default|GetdebugCube)))

(event EventBeginPlay
  (bind _scenecapturecomponent2d (Variables|Default|GetSceneCaptureComponent2D))
  (bind _debugcube (Variables|Default|GetdebugCube))
  (bind _returnvalue (Transformation|GetActorLocation _debugcube))
  (bind _orthowidth (Variables|/Script/Engine.SceneCaptureComponent2D|GetOrthoWidth _scenecapturecomponent2d))
  (bind (_x _y) (Class|KismetMathLibrary|BreakVector3f _returnvalue))
  (bind _returnvalue_2 (/ _orthowidth 2.0))
  (Variables|/Script/Engine.PlayerController|SetbShowMouseCursor (Game|GetPlayerController 0) true)
  (bind _returnvalue_3 (UserInterface|CreateWidget "/Game/ProjetFilRouge/Core/Mobile/MiniMap/WBP_MiniMap.WBP_MiniMap_C" (Game|GetPlayerController 0)))
  (bind _output_get (Variables|Default|Setminimap _returnvalue_3))
  (UserInterface|Viewport|AddtoPlayerScreen _output_get)
  (bind _returnvalue_4 (UserInterface|CreateWidget "/Game/ProjetFilRouge/Core/Mobile/MiniMap/WBP_MiniMap_MapButton.WBP_MiniMap_MapButton_C"))
  (bind _output_get_2 (Variables|Default|SettestCursor _returnvalue_4))
  (UserInterface|Viewport|AddtoPlayerScreen _output_get_2)
  (bind _returnvalue_5 (Class|Overlay|AddChildtoOverlay (Variables|/Game/ProjetFilRouge/Core/Mobile/MiniMap/WBP_MiniMap.WBP_MiniMap_C|GetMapOverlay (Variables|Default|Getminimap)) _returnvalue_4))
  (Layout|GridSlot|SetHorizontalAlignment _returnvalue_5 "HAlign_Center")
  (Layout|GridSlot|SetVerticalAlignment _returnvalue_5 "VAlign_Center")
  (EventDispatchers|BindEventtoOnButtonClicked _output_get_2 (delegate Custom|DeleteActor))
  (Class|Widget|SetRenderTranslation (Variables|Default|GettestCursor) (Math|Vector2D|MakeVector2D (* (/ _y _returnvalue_2) (/ (.X (Math|Vector2D|BreakVector2D (Class|CanvasPanelSlot|GetSize (Class|WidgetLayoutLibrary|SlotasCanvasSlot (Variables|/Game/ProjetFilRouge/Core/Mobile/MiniMap/WBP_MiniMap.WBP_MiniMap_C|GetMiniMap (Variables|Default|Getminimap)))))) 2.0)) (* (* (/ _x _returnvalue_2) (/ (.X (Math|Vector2D|BreakVector2D (Class|CanvasPanelSlot|GetSize (Class|WidgetLayoutLibrary|SlotasCanvasSlot (Variables|/Game/ProjetFilRouge/Core/Mobile/MiniMap/WBP_MiniMap.WBP_MiniMap_C|GetMiniMap (Variables|Default|Getminimap)))))) 2.0)) -1.0))))

(fn ConstructionScript)